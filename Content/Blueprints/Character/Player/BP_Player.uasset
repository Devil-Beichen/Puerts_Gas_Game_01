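; BP_Player is the player character Blueprint, wiring player input to movement, look, jump and camera lock actions.
; Enhanced Input events pass move and look values to Move and Look, while the jump action calls Jump on start.
; A FlipFlop on the V key toggles LockCamera on and off.
; Move, Look and LockCamera have empty bodies here, and BeginPlay only calls its parent and EmptyFunction.
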(event `self.ReceiveBeginPlay`
  (`parent.ReceiveBeginPlay`)
  (`GasFunctionLibrary.EmptyFunction`))

(event `EnhancedInput|/Game/Blueprints/Input/Action/IA_Move`
  (params (ActionValue :type "Vector2D Structure") (ElapsedSeconds :type "Float (double-precision)") (TriggeredSeconds :type "Float (double-precision)") (InputAction :type "InputAction Object Reference" :default "/Game/Blueprints/Input/Action/IA_Move.IA_Move"))
  (:`Triggered`
    (`self.Move` ActionValue)))

(event `EnhancedInput|/Game/Blueprints/Input/Action/IA_Look`
  (params (ActionValue :type "Vector2D Structure") (ElapsedSeconds :type "Float (double-precision)") (TriggeredSeconds :type "Float (double-precision)") (InputAction :type "InputAction Object Reference" :default "/Game/Blueprints/Input/Action/IA_Look.IA_Look"))
  (:`Triggered`
    (`self.Look` ActionValue)))

(event `EnhancedInput|/Game/Blueprints/Input/Action/IA_Jump`
  (params (ActionValue :type Boolean) (ElapsedSeconds :type "Float (double-precision)") (TriggeredSeconds :type "Float (double-precision)") (InputAction :type "InputAction Object Reference" :default "/Game/Blueprints/Input/Action/IA_Jump.IA_Jump"))
  (:`Started`
    (`self.Jump`)))

(event `Key|V`
  (params (Key :type "Key Structure"))
  (:`Pressed`
    (`/Engine/EditorBlueprintResources/StandardMacros.FlipFlop`
      (:`A`
        (`self.LockCamera` true))
      (:`B`
        (`self.LockCamera` false)))))

(fn `LockCamera`
  (params (`Lock?` :type Boolean)))

(fn `Look`
  (params (ActionValue :type "Vector2D Structure")))

(fn `Move`
  (params (ActionValue :type "Vector2D Structure")))

(fn `UserConstructionScript`
  (`parent.UserConstructionScript`))